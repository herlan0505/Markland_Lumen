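; An hourglass light fixture, filed with the sconce lights, that toggles on and off when interacted with.
; Both spot lights are made visible at BeginPlay, and a FlipFlop on the Interact event alternates between the off and on functions, starting with off.
; Each function sets the lights' visibility, swaps the bulb material slot on the mesh and plays a toggle sound at its location.
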(event `self.ReceiveBeginPlay`
  (`SceneComponent.SetVisibility` (`self.SpotLight1`) true false)
  (`SceneComponent.SetVisibility` (`self.SpotLight`) true false))

(event `/Game/FirstPerson/Blueprints/Herlan_Blueprint/interact/BP_Interact.BP_interact`
  ;[0 0.04421 1 0.5] Toggle light
  (`/Engine/EditorBlueprintResources/StandardMacros.FlipFlop`
    (:`A`
      (`self.islight Off?`))
    (:`B`
      (`self.islight On?`))))

(fn `islight Off?`
  (`SceneComponent.SetVisibility` (`self.SpotLight1`) false false)
  (`SceneComponent.SetVisibility` (`self.SpotLight`) false false)
  (`PrimitiveComponent.SetMaterial` (`self.sm_light_hourglass`) 2 "/Game/_Addons/Fixtures/MI_WhiteBulb.MI_WhiteBulb")
  (`GameplayStatics.PlaySoundAtLocation` "/Game/FirstPerson/Blueprints/Herlan_Blueprint/sound/ToggleLamp.ToggleLamp" (`SceneComponent.K2_GetComponentLocation` (`self.sm_light_hourglass`)) (struct) 1.0 1.0 0.0 null null null null))

(fn `islight On?`
  (`SceneComponent.SetVisibility` (`self.SpotLight1`) true false)
  (`SceneComponent.SetVisibility` (`self.SpotLight`) true false)
  (`PrimitiveComponent.SetMaterial` (`self.sm_light_hourglass`) 2 "/Game/_Addons/Fixtures/SconeLights/Light_Hourglass/Materials/Material__33.Material__33")
  (`GameplayStatics.PlaySoundAtLocation` "/Game/FirstPerson/Blueprints/Herlan_Blueprint/sound/ToggleLamp.ToggleLamp" (`SceneComponent.K2_GetComponentLocation` (`self.sm_light_hourglass`)) (struct) 1.0 1.0 0.0 null null null null))

(fn `UserConstructionScript`)