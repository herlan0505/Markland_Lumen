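; Wall sconce light fixture actor that can be switched on and off.
; An Interact event flips LightOn and calls the on or off function, which toggles the spotlight's visibility and swaps two bulb material slots between lit and unlit glass.
; SetLightState applies the same changes from an IsNight flag, so external logic can set the light by time of day.
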(event `/Game/FirstPerson/Blueprints/Herlan_Blueprint/interact/BP_Interact.BP_interact`
  ; toggle light
  (bind _output_get (set `self.Light on` (not (`self.Light on`))))
  (if _output_get
    (`self.islight on?`)
    (else
      (`self.islight off?`))))

(fn `islight off?`
  (bind _staticmesh (`self.StaticMesh`))
  (bind _output_get (set `self.Light on` false))
  (if (not _output_get)
    (`SceneComponent.SetVisibility` (`self.SpotLight1`) false false)
    (`|ExecutionSequence`
      (:`then_0`
        (`PrimitiveComponent.SetMaterial` _staticmesh 1 "/Game/_Addons/Fixtures/SconeLights/crispscone/M_FakeGlassOff.M_FakeGlassOff")
        (`PrimitiveComponent.SetMaterial` _staticmesh 2 "/Game/_Addons/Fixtures/SconeLights/crispscone/M_FakeGlassOff.M_FakeGlassOff")))))

(fn `islight on?`
  (bind _staticmesh (`self.StaticMesh`))
  (bind _output_get (set `self.Light on` true))
  (if _output_get
    (`SceneComponent.SetVisibility` (`self.SpotLight1`) true false)
    (`|ExecutionSequence`
      (:`then_0`
        (`PrimitiveComponent.SetMaterial` _staticmesh 1 "/Game/_Addons/Fixtures/SconeLights/crispscone/MI_FakeGlassBulbOn.MI_FakeGlassBulbOn")
        (`PrimitiveComponent.SetMaterial` _staticmesh 2 "/Game/_Addons/Fixtures/SconeLights/crispscone/MI_FakeGlassBulbOn.MI_FakeGlassBulbOn")))))

(fn `set light state`
  (params (`is night` :type Boolean))
  (bind _staticmesh (`self.StaticMesh`))
  (bind _staticmesh_2 (`self.StaticMesh`))
  (bind _output_get (set `self.Light on` `is night`))
  (if _output_get
    (`SceneComponent.SetVisibility` (`self.SpotLight1`) true false)
    (`PrimitiveComponent.SetMaterial` _staticmesh_2 1 "/Game/_Addons/Fixtures/SconeLights/crispscone/MI_FakeGlassBulbOn.MI_FakeGlassBulbOn")
    (`PrimitiveComponent.SetMaterial` _staticmesh_2 2 "/Game/_Addons/Fixtures/SconeLights/crispscone/MI_FakeGlassBulbOn.MI_FakeGlassBulbOn")
    (else
      (`SceneComponent.SetVisibility` (`self.SpotLight1`) false false)
      (`|ExecutionSequence`
        (:`then_0`
          (`PrimitiveComponent.SetMaterial` _staticmesh 1 "/Game/_Addons/Fixtures/SconeLights/crispscone/M_FakeGlassOff.M_FakeGlassOff")
          (`PrimitiveComponent.SetMaterial` _staticmesh 2 "/Game/_Addons/Fixtures/SconeLights/crispscone/M_FakeGlassOff.M_FakeGlassOff"))))))

(fn `UserConstructionScript`)