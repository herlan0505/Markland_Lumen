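; BP_PotLight is an interactable potlight fixture that players can switch on and off.
; The Interact event flips LightOn and calls IsLightOn or IsLightOff, which set the spotlight's visibility and swap the fixture mesh material between an LED material and plain white.
; The construction script matches spotlight visibility to LightOn, but leaves the mesh material untouched.
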(event `self.ReceiveBeginPlay`)

(event `/Game/FirstPerson/Blueprints/Herlan_Blueprint/interact/BP_Interact.BP_interact`
  ; Toggle light
  (bind _output_get (set `self.Light on` (not (`self.Light on`))))
  (if _output_get
    (`self.isLight On?`)
    (else
      (`self.isLight Off?`))))

(fn `isLight Off?`
  (bind _output_get (set `self.Light on` false))
  (if (not _output_get)
    (`SceneComponent.SetVisibility` (`self.SpotLight`) false false)
    (`PrimitiveComponent.SetMaterial` (`self.SM_PotLight`) 0 "/Game/Herlan/white.white")))

(fn `isLight On?`
  (bind _output_get (set `self.Light on` true))
  (if _output_get
    (`SceneComponent.SetVisibility` (`self.SpotLight`) true false)
    (`PrimitiveComponent.SetMaterial` (`self.SM_PotLight`) 0 "/Game/Megascans/BrandColors/MI_LightLED02.MI_LightLED02")))

(fn `UserConstructionScript`
  (`SceneComponent.SetVisibility` (`self.SpotLight`) (`self.Light on`) false))