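; BP_StairLight is a stair light fixture that switches on and off when it receives an Interact event.
; Interact flips the LightOn flag and calls IslightOn or IsLightOff.
; Each function sets the flag again, shows or hides the SpotLight, and swaps the mesh's first material between the lit and unlit white bulb instances.
; Construction script, BeginPlay and Tick are empty, so nothing applies the initial state.
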(event `/Game/FirstPerson/Blueprints/Herlan_Blueprint/interact/BP_Interact.BP_interact`
  ; toggle
  (bind _output_get (set `self.Light on` (not (`self.Light on`))))
  (if _output_get
    (`self.Islight on?`)
    (else
      (`self.isLight off?`))))

(fn `isLight off?`
  (bind _output_get (set `self.Light on` false))
  (if (not _output_get)
    (`SceneComponent.SetVisibility` (`self.SpotLight`) false false)
    (`PrimitiveComponent.SetMaterial` (`self.SM_StairLight`) 0 "/Game/_Addons/Fixtures/MI_WhiteBulbOff.MI_WhiteBulbOff")))

(fn `Islight on?`
  (bind _output_get (set `self.Light on` true))
  (if _output_get
    (`SceneComponent.SetVisibility` (`self.SpotLight`) true false)
    (`PrimitiveComponent.SetMaterial` (`self.SM_StairLight`) 0 "/Game/_Addons/Fixtures/MI_WhiteBulbOn.MI_WhiteBulbOn")))

(fn `UserConstructionScript`)