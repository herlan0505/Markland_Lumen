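; Bowl shade pendant light fixture that toggles off and on through its Interact event.
; A FlipFlop alternates between turning the spotlight off with a plain white material on the lamp mesh and restoring its intensity with the bulb material.
; The first interaction switches it off.
; Toggle sound nodes are present but disconnected, so switching plays no sound.
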(event `/Game/FirstPerson/Blueprints/Herlan_Blueprint/interact/BP_Interact.BP_interact`
  (`/Engine/EditorBlueprintResources/StandardMacros.FlipFlop`
    (:`A`
      (`|ExecutionSequence`
        (:`then_0`
          (`LightComponent.SetIntensity` (`self.SpotLight`) 0.0))
        (:`then_1`
          (`PrimitiveComponent.SetMaterial` (`self.SM_BowlShadeLight_Lamp`) 0 "/Game/Herlan/white.white"))))
    (:`B`
      (`|ExecutionSequence`
        (:`then_0`
          (`LightComponent.SetIntensity` (`self.SpotLight`) 250.0))
        (:`then_1`
          (`PrimitiveComponent.SetMaterial` (`self.SM_BowlShadeLight_Lamp`) 0 "/Game/_Addons/Fixtures/MI_WhiteBulb.MI_WhiteBulb"))))))

(fn `UserConstructionScript`)