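; Bowl-shade pendant light fixture that toggles on and off when interacted with.
; The Interact event runs a FlipFlop, switching the light off on the first call and on at the next.
; The IslightOn and IslightOff functions set SpotLight visibility and swap the lamp mesh's first material slot between MI_WhiteBulb for on and M_WhiteBulb for off.
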(event `self.BP_interact`
  (`/Engine/EditorBlueprintResources/StandardMacros.FlipFlop`
    (:`A`
      (`self.islight Off?`))
    (:`B`
      (`self.islight On?`))))

(fn `islight Off?`
  (`SceneComponent.SetVisibility` (`self.SpotLight`) false false)
  (`PrimitiveComponent.SetMaterial` (`self.SM_BowlShadeLight_Lamp`) 0 "/Game/_Addons/Fixtures/M_WhiteBulb.M_WhiteBulb"))

(fn `islight On?`
  (`SceneComponent.SetVisibility` (`self.SpotLight`) true false)
  (`PrimitiveComponent.SetMaterial` (`self.SM_BowlShadeLight_Lamp`) 0 "/Game/_Addons/Fixtures/MI_WhiteBulb.MI_WhiteBulb"))

(fn `UserConstructionScript`)