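; BP_PENDANT03 is an interactable Japanese-style pendant light fixture that can be switched on and off.
; Interact alternates through a FlipFlop, turning the light off first, with each state setting SpotLight visibility and swapping a mesh material between glowing-bulb and plain fake glass.
; An icon widget starts hidden, is toggled by ShowIcon and HideIcon, and rotates every tick to face the player camera.
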(event `self.ReceiveTick`
  (params (DeltaSeconds :type "Float (single-precision)"))
  (bind _widget (`self.Widget`))
  ; widget follow camera
  (`SceneComponent.K2_SetWorldRotation` _widget (`KismetMathLibrary.FindLookAtRotation` (`SceneComponent.K2_GetComponentLocation` _widget) (`SceneComponent.K2_GetComponentLocation` (`PlayerCameraManager.TransformComponent` (`GameplayStatics.GetPlayerCameraManager` 0)))) false false))

(event `self.ReceiveBeginPlay`
  (`SceneComponent.SetVisibility` (`self.Widget`) false false))

(event `/Game/FirstPerson/Blueprints/Herlan_Blueprint/interact/BP_Interact.BP_interact`
  ;[0.02439 0.03179 1 0.5] Toggle Light
  (`/Engine/EditorBlueprintResources/StandardMacros.FlipFlop`
    (:`A`
      (`self.islight Off`))
    (:`B`
      (`self.islight On ?`))))

(event `/Game/FirstPerson/Blueprints/Herlan_Blueprint/interact/BPI_Interact.Hide icon`
  ; widget visibility
  (`SceneComponent.SetVisibility` (`self.Widget`) false false))

(event `/Game/FirstPerson/Blueprints/Herlan_Blueprint/interact/BPI_Interact.Show icon`
  ; widget visibility
  (`SceneComponent.SetVisibility` (`self.Widget`) true false))

(fn `islight Off`
  (`SceneComponent.SetVisibility` (`self.SpotLight`) false false)
  (`PrimitiveComponent.SetMaterial` (`self.StaticMesh`) 2 "/Game/_Addons/Fixtures/SconeLights/crispscone/M_FakeGlass.M_FakeGlass"))

(fn `islight On ?`
  (`SceneComponent.SetVisibility` (`self.SpotLight`) true false)
  (`PrimitiveComponent.SetMaterial` (`self.StaticMesh`) 2 "/Game/_Addons/Fixtures/SconeLights/crispscone/MI_FakeGlassBulb.MI_FakeGlassBulb"))

(fn `UserConstructionScript`)