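; Flush-mount ceiling light actor that the player can toggle through an Interact event.
; A FlipFlop alternates between the off and on functions, starting with off, each setting spotlight visibility, swapping the fabric material and playing a toggle sound at the mesh.
; An icon widget starts hidden, is shown or hidden by ShowIcon and HideIcon, and rotates every tick to face the player camera.
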(event `self.ReceiveBeginPlay`
  (`SceneComponent.SetVisibility` (`self.Widget`) false false))

(event `/Game/FirstPerson/Blueprints/Herlan_Blueprint/interact/BP_Interact.BP_interact`
  ; toggle light
  (`/Engine/EditorBlueprintResources/StandardMacros.FlipFlop`
    (:`A`
      (`self.islight Off?`))
    (:`B`
      (`self.islight On?`))))

(event `self.ReceiveTick`
  (params (DeltaSeconds :type "Float (single-precision)"))
  (bind _widget (`self.Widget`))
  (`SceneComponent.K2_SetWorldRotation` _widget (`KismetMathLibrary.FindLookAtRotation` (`SceneComponent.K2_GetComponentLocation` _widget) (`SceneComponent.K2_GetComponentLocation` (`PlayerCameraManager.TransformComponent` (`GameplayStatics.GetPlayerCameraManager` 0)))) false false))

(event `/Game/FirstPerson/Blueprints/Herlan_Blueprint/interact/BPI_Interact.Hide icon`
  ; widet visibility
  (`SceneComponent.SetVisibility` (`self.Widget`) false false))

(event `/Game/FirstPerson/Blueprints/Herlan_Blueprint/interact/BPI_Interact.Show icon`
  ; widet visibility
  (`SceneComponent.SetVisibility` (`self.Widget`) true false))

(fn `islight Off?`
  (`SceneComponent.SetVisibility` (`self.spotlight`) false false)
  (`PrimitiveComponent.SetMaterial` (`self.StaticMesh`) 0 "/Game/_Addons/Fixtures/FlushMountLight/RestorationHardwareLight/MI_LightFabric1.MI_LightFabric1")
  (`GameplayStatics.PlaySoundAtLocation` "/Game/FirstPerson/Blueprints/Herlan_Blueprint/sound/ToggleLamp.ToggleLamp" (`SceneComponent.K2_GetComponentLocation` (`self.StaticMesh`)) (struct) 1.0 1.0 0.0 null null null null))

(fn `islight On?`
  (`SceneComponent.SetVisibility` (`self.spotlight`) true false)
  (`PrimitiveComponent.SetMaterial` (`self.StaticMesh`) 0 "/Game/_Addons/Fixtures/FlushMountLight/RestorationHardwareLight/MI_LightFabric.MI_LightFabric")
  (`GameplayStatics.PlaySoundAtLocation` "/Game/FirstPerson/Blueprints/Herlan_Blueprint/sound/ToggleLamp.ToggleLamp" (`SceneComponent.K2_GetComponentLocation` (`self.StaticMesh`)) (struct) 1.0 1.0 0.0 null null null null))

(fn `UserConstructionScript`)