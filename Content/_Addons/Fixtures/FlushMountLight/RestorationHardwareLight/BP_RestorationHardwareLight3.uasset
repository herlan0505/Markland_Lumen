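; Flush-mount ceiling light fixture Blueprint that the player can switch on and off through an Interact event.
; A FlipFlop alternates between two functions on each interaction, turning the light off first.
; Each function sets the spotlight's visibility and swaps the mesh's first material between lit and unlit fabric to match.
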(event `self.BP_interact`
  (`/Engine/EditorBlueprintResources/StandardMacros.FlipFlop`
    (:`A`
      (`self.islight Off?`))
    (:`B`
      (`self.islight On?`))))

(fn `islight Off?`
  (`SceneComponent.SetVisibility` (`self.spotlight`) false false)
  (`PrimitiveComponent.SetMaterial` (`self.StaticMesh`) 0 "/Game/_Addons/Fixtures/FlushMountLight/RestorationHardwareLight/MI_LightFabricOff.MI_LightFabricOff"))

(fn `islight On?`
  (`SceneComponent.SetVisibility` (`self.spotlight`) true false)
  (`PrimitiveComponent.SetMaterial` (`self.StaticMesh`) 0 "/Game/_Addons/Fixtures/FlushMountLight/RestorationHardwareLight/MI_LightFabricON.MI_LightFabricON"))

(fn `UserConstructionScript`)