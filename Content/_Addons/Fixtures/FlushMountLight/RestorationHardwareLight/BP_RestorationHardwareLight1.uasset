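; Interactable flush-mount ceiling light Blueprint that the player can toggle on and off.
; Interact flips LightOn, which shows or hides the spotlight and swaps the fixture's fabric material between lit and unlit versions.
; An icon widget starts hidden, is toggled by ShowIcon and HideIcon, and turns every Tick to face the player camera.
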(event `self.ReceiveBeginPlay`
  (`SceneComponent.SetVisibility` (`self.Widget`) false false))

(event `/Game/FirstPerson/Blueprints/Herlan_Blueprint/interact/BP_Interact.BP_interact`
  ; toggle light
  (bind _output_get (set `self.Light on` (not (`self.Light on`))))
  (if _output_get
    (`self.islight On?`)
    (else
      (`self.islight Off?`))))

(event `/Game/FirstPerson/Blueprints/Herlan_Blueprint/interact/BPI_Interact.Hide icon`
  ; widget visibility
  (`SceneComponent.SetVisibility` (`self.Widget`) false false))

(event `self.ReceiveTick`
  (params (DeltaSeconds :type "Float (single-precision)"))
  (bind _widget (`self.Widget`))
  ; widget follow camera
  (`SceneComponent.K2_SetWorldRotation` _widget (`KismetMathLibrary.FindLookAtRotation` (`SceneComponent.K2_GetComponentLocation` _widget) (`SceneComponent.K2_GetComponentLocation` (`PlayerCameraManager.TransformComponent` (`GameplayStatics.GetPlayerCameraManager` 0)))) false false))

(event `/Game/FirstPerson/Blueprints/Herlan_Blueprint/interact/BPI_Interact.Show icon`
  ; widget visibility
  (`SceneComponent.SetVisibility` (`self.Widget`) true false))

(fn `islight Off?`
  (bind _output_get (set `self.Light on` false))
  (if (not _output_get)
    (`SceneComponent.SetVisibility` (`self.spotlight`) false false)
    (`PrimitiveComponent.SetMaterial` (`self.StaticMesh`) 0 "/Game/_Addons/Fixtures/FlushMountLight/RestorationHardwareLight/MI_LightFabricOff.MI_LightFabricOff")))

(fn `islight On?`
  (bind _output_get (set `self.Light on` true))
  (if _output_get
    (`SceneComponent.SetVisibility` (`self.spotlight`) true false)
    (`PrimitiveComponent.SetMaterial` (`self.StaticMesh`) 0 "/Game/_Addons/Fixtures/FlushMountLight/RestorationHardwareLight/MI_LightFabricON.MI_LightFabricON")))

(fn `UserConstructionScript`)