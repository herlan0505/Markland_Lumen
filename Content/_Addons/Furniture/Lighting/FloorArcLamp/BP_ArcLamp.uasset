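; BP_ArcLamp is an interactable floor arc lamp that can be switched on and off.
; Interact flips LightOn and calls a helper function that shows or hides the Ee component to match.
; An icon Widget starts hidden, is toggled by ShowIcon and HideIcon, and rotates every Tick to face the player camera.
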(event `self.ReceiveBeginPlay`
  (`SceneComponent.SetVisibility` (`self.Widget`) false false))

(event `self.ReceiveTick`
  (params (DeltaSeconds :type "Float (single-precision)"))
  (bind _widget (`self.Widget`))
  ; widget follow camera
  (`SceneComponent.K2_SetWorldRotation` _widget (`KismetMathLibrary.FindLookAtRotation` (`SceneComponent.K2_GetComponentLocation` _widget) (`SceneComponent.K2_GetComponentLocation` (`PlayerCameraManager.TransformComponent` (`GameplayStatics.GetPlayerCameraManager` 0)))) false false))

(event `/Game/FirstPerson/Blueprints/Herlan_Blueprint/interact/BP_Interact.BP_interact`
  ; Toggle Lamp
  (bind _output_get (set `self.Light on` (not (`self.Light on`))))
  (if _output_get
    (`self.isLIght On?`)
    (else
      (`self.isLight Off?`))))

(event `/Game/FirstPerson/Blueprints/Herlan_Blueprint/interact/BPI_Interact.Hide icon`
  ; Widget visibility
  (`SceneComponent.SetVisibility` (`self.Widget`) false false))

(event `/Game/FirstPerson/Blueprints/Herlan_Blueprint/interact/BPI_Interact.Show icon`
  ; Widget visibility
  (`SceneComponent.SetVisibility` (`self.Widget`) true false))

(fn `isLight Off?`
  (bind _output_get (set `self.Light on` false))
  (if (not _output_get)
    (`SceneComponent.SetVisibility` (`self.ee`) false false)))

(fn `isLIght On?`
  (bind _output_get (set `self.Light on` true))
  (if _output_get
    (`SceneComponent.SetVisibility` (`self.ee`) true false)))

(fn `UserConstructionScript`)