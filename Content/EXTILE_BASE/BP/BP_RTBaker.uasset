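; BP_RTBaker is a Blueprint utility that bakes a material into a render target and exports the result to a file.
; Its Bake event clears the target to opaque black, draws the material into it, then exports it with the configured path and file name.
; The construction script calls Bake whenever the BakeToRenderTarget flag is set, so the bake runs on construction without any gameplay logic.
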(event `Bake`
  (bind _rendertarget (`self.RenderTarget`))
  (`KismetRenderingLibrary.ClearRenderTarget2D` _rendertarget)
  (`KismetRenderingLibrary.DrawMaterialToRenderTarget` _rendertarget (`self.Material`))
  (`KismetRenderingLibrary.ExportRenderTarget` _rendertarget (`self.Export (File Path)`) (`self.File Name`)))

(fn `UserConstructionScript`
  (if (`self.Bake to Render Target?`)
    (`self.Bake`)))